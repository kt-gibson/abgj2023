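; BP_TestCharacter is a test player character that moves with Enhanced Input and can grab overlapped enemies.
; On BeginPlay it adds the IMC_Reach mapping context, and IA_Move drives movement relative to control yaw.
; Overlapping a Character whose capsule has the "Enemy" tag sets an overlap flag, which lets IA_Grab attach the last overlapped actor to itself.
; Any end overlap clears the flag, and debug prints report collisions and failed casts.
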(event Input|EnhancedActionEvents|EnhancedInputActionIA_Move
  (params (ActionValue :type Vector%202D%20Structure) (ElapsedSeconds :type Float%20%28double-precision%29) (TriggeredSeconds :type Float%20%28double-precision%29) (InputAction :type Input%20Action%20Object%20Reference :default "/Game/Input/IA_Move.IA_Move"))
  (bind _returnvalue (Pawn|GetControlRotation :!class /Script/Engine.Pawn))
  ;[1 1 1] Set up movement input listener
  (:Triggered
    (Pawn|Input|AddMovementInput (Math|Vector|GetRightVector (Math|Rotator|MakeRotator (.roll _returnvalue) 0.0 (.yaw _returnvalue))) (.x ActionValue) false)
    (Pawn|Input|AddMovementInput (Math|Vector|GetForwardVector (Math|Rotator|MakeRotator 0.0 0.0 (.yaw (Pawn|GetControlRotation :!class /Script/Engine.Pawn)))) (.y ActionValue) false)))

(event Input|EnhancedActionEvents|EnhancedInputActionIA_Grab
  (params (ActionValue :type Boolean) (ElapsedSeconds :type Float%20%28double-precision%29) (TriggeredSeconds :type Float%20%28double-precision%29) (InputAction :type Input%20Action%20Object%20Reference :default "/Game/Input/IA_Grab.IA_Grab"))
  (:Triggered
    (if (Variables|Default|GetIsOverlapped)
      (Transformation|AttachActorToActor (Variables|Default|GetOther%20Actor) self "None" "KeepWorld" "KeepRelative" "KeepRelative" true))))

(event EventBeginPlay
  ;[1 1 1] Set up enhanced input
  (bind _asplayer_controller (Utilities|Casting|CastToPlayerController (Pawn|GetController)))
  (Utilities|IsValid (PlayerController|LocalPlayerSubsystems|GetEnhancedInputLocalPlayerSubsystem _asplayer_controller)
    (:Is%20Valid
      (Input|AddMappingContext (PlayerController|LocalPlayerSubsystems|GetEnhancedInputLocalPlayerSubsystem _asplayer_controller) "/Game/Input/IMC_Reach.IMC_Reach" 0 "(bIgnoreAllPressedKeysUntilRelease=True,bForceImmediately=False)"))))

(event Collision|EventActorBeginOverlap
  (params (OtherActor :type Actor%20Object%20Reference))
  (bind _output_get (Variables|Default|SetOther%20Actor OtherActor))
  (bind _ascharacter (Utilities|Casting|CastToCharacter _output_get)
    (:then
      (if (Components|ComponentHasTag (Variables|/Script/Engine.Character|GetCapsuleComponent _ascharacter) "Enemy")
        (Development|PrintString "COLLIDED WITH ENEMY!")
        (Variables|Default|SetIsOverlapped true)))
    (:CastFailed
      (Development|PrintString "CAST FAILED"))))

(event EventTick
  (params (DeltaSeconds :type Float%20%28single-precision%29)))

(event Collision|EventActorEndOverlap
  (params (OtherActor :type Actor%20Object%20Reference))
  (Variables|Default|SetIsOverlapped false))

(fn ConstructionScript)